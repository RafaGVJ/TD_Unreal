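; BP_TP is a one-way teleporter that moves the player character from entrance box Ent to exit box Ext.
; On overlap with Ent, it re-expresses the player's transform relative to Ent in Ext's space, preserving relative position and orientation.
; The construction script sizes both boxes from a shared BoxSize so they match.
; A coin sound node is present but unconnected.
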(event OnComponentBeginOverlap(Ent)
  (params (OverlappedComponent :type Primitive%20Component%20Object%20Reference) (OtherActor :type Actor%20Object%20Reference) (OtherComp :type Primitive%20Component%20Object%20Reference) (OtherBodyIndex :type Integer) (bFromSweep :type Boolean) (SweepResult :type Hit%20Result%20Structure%20%28by%20ref%29))
  (if (== OtherActor (Game|GetPlayerCharacter 0))
    (Transformation|SetActorTransform (Game|GetPlayerCharacter 0) (CallFunction|GetDestinationTransform))))

(fn ConstructionScript
  (Components|Box|SetBoxExtent (Variables|Default|GetEnt) (Variables|Default|GetBoxSize) true))

(fn GetDestinationTransform
  (return (Math|Transform|ComposeTransforms (Math|Transform|MakeRelativeTransform (Transformation|GetActorTransform (Game|GetPlayerCharacter 0)) (Transformation|GetWorldTransform (Variables|Default|GetEnt))) (Transformation|GetWorldTransform (Variables|Default|GetExt)))))